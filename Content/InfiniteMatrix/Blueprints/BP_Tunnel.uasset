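; BP_Tunnel is a tunnel segment with a spinning obstacle wall that the player must pass.
; RandomizeWall picks one of twenty hole meshes and gives the wall a random roll; Tick keeps it rotating.
; Clearing the trigger adds score, while hitting the wall costs health and, at zero, marks the player dead and shows restart.
; Either contact asks TunnelSpawner for a new tunnel and destroys this one.
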(event `self.ReceiveTick`
  (params (DeltaSeconds :type "Float (single-precision)"))
  (`SceneComponent.K2_AddLocalRotation` (`self.WallMesh`) (`KismetMathLibrary.MakeRotator` (* DeltaSeconds (`self.RotateSpeed`))) false false))

(event `self.TriggerZone.OnComponentBeginOverlap`
  (params (OverlappedComponent :type "PrimitiveComponent Object Reference") (OtherActor :type "Actor Object Reference") (OtherComp :type "PrimitiveComponent Object Reference") (OtherBodyIndex :type Integer) (bFromSweep :type Boolean) (SweepResult :type "HitResult Structure (by ref)"))
  (bind _asbp_player (cast `/Game/InfiniteMatrix/Blueprints/BP_Player` OtherActor))
  (set `/Game/InfiniteMatrix/Blueprints/BP_Player.Score` (+ (`/Game/InfiniteMatrix/Blueprints/BP_Player.Score` _asbp_player) 1.0) _asbp_player)
  (`/Game/InfiniteMatrix/Blueprints/BP_TunnelSpawner.SpawnTunnelAtSpawnPoint` (`self.TunnelSpawner`))
  (`self.K2_DestroyActor`))

(event `self.WallMesh.OnComponentHit`
  (params (HitComponent :type "PrimitiveComponent Object Reference") (OtherActor :type "Actor Object Reference") (OtherComp :type "PrimitiveComponent Object Reference") (NormalImpulse :type "Vector Structure") (Hit :type "HitResult Structure (by ref)"))
  (bind _asbp_player (cast `/Game/InfiniteMatrix/Blueprints/BP_Player` OtherActor))
  (set `/Game/InfiniteMatrix/Blueprints/BP_Player.Health` (`KismetMathLibrary.FClamp` (- (`/Game/InfiniteMatrix/Blueprints/BP_Player.Health` _asbp_player) 50.0) 0.0 100.0) _asbp_player)
  (`/Game/InfiniteMatrix/Blueprints/BP_TunnelSpawner.SpawnTunnelAtSpawnPoint` (`self.TunnelSpawner`))
  (`self.K2_DestroyActor`)
  (if (== (`/Game/InfiniteMatrix/Blueprints/BP_Player.Health` _asbp_player) 0.0)
    (set `/Game/InfiniteMatrix/Blueprints/BP_Player.IsDead` true _asbp_player)
    (set `/Game/InfiniteMatrix/Blueprints/BP_Player.ForwardSpeed` 2000.0 _asbp_player)
    (`/Game/InfiniteMatrix/Blueprints/BP_Player.DisplayRestart` _asbp_player)))

(fn `RandomizeWall`
  (`StaticMeshComponent.SetStaticMesh` (`self.WallMesh`) (select `int` (`KismetMathLibrary.RandomIntegerInRange` 0 19) :`0` "/Game/InfiniteMatrix/Meshes/SM_Hole_01.SM_Hole_01" :`1` "/Game/InfiniteMatrix/Meshes/SM_Hole_02.SM_Hole_02" :`2` "/Game/InfiniteMatrix/Meshes/SM_Hole_03.SM_Hole_03" :`3` "/Game/InfiniteMatrix/Meshes/SM_Hole_04.SM_Hole_04" :`4` "/Game/InfiniteMatrix/Meshes/SM_Hole_05.SM_Hole_05" :`5` "/Game/InfiniteMatrix/Meshes/SM_Hole_06.SM_Hole_06" :`6` "/Game/InfiniteMatrix/Meshes/SM_Hole_07.SM_Hole_07" :`7` "/Game/InfiniteMatrix/Meshes/SM_Hole_08.SM_Hole_08" :`8` "/Game/InfiniteMatrix/Meshes/SM_Hole_09.SM_Hole_09" :`9` "/Game/InfiniteMatrix/Meshes/SM_Hole_10.SM_Hole_10" :`10` "/Game/InfiniteMatrix/Meshes/SM_Hole_11.SM_Hole_11" :`11` "/Game/InfiniteMatrix/Meshes/SM_Hole_12.SM_Hole_12" :`12` "/Game/InfiniteMatrix/Meshes/SM_Hole_13.SM_Hole_13" :`13` "/Game/InfiniteMatrix/Meshes/SM_Hole_14.SM_Hole_14" :`14` "/Game/InfiniteMatrix/Meshes/SM_Hole_15.SM_Hole_15" :`15` "/Game/InfiniteMatrix/Meshes/SM_Hole_16.SM_Hole_16" :`16` "/Game/InfiniteMatrix/Meshes/SM_Hole_17.SM_Hole_17" :`17` "/Game/InfiniteMatrix/Meshes/SM_Hole_18.SM_Hole_18" :`18` "/Game/InfiniteMatrix/Meshes/SM_Hole_19.SM_Hole_19" :`19` "/Game/InfiniteMatrix/Meshes/SM_Hole_20.SM_Hole_20" :!type "StaticMesh Object Reference"))
  (`SceneComponent.K2_AddLocalRotation` (`self.WallMesh`) (`KismetMathLibrary.MakeRotator` (`KismetMathLibrary.RandomFloatInRange` 0.0 360.0)) false false))

(fn `UserConstructionScript`)